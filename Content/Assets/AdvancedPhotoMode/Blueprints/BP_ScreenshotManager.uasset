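; BP_ScreenshotManager is a photo mode actor that captures and exports a screenshot at a requested size, ticking while paused.
; TakeScreenshot adds a scene capture with the current post process and FOV, rendering into a new render target.
; After a time-dilation-scaled delay, it exports the image, toggling logo colors around the export.
; A FlipFlop makes a thumbnail on the first call, then registers and destroys the actor on the second.
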(event Custom|TakeScreenshot
  (params (Size :type Int%20Point%20Structure) (Path :type String) (Filename :type String))
  (bind (_x _y) (Utilities|Struct|BreakIntPoint Size))
  (bind _photomodewidgetref (Variables|Default|GetPhotoModeWidgetRef))
  (bind _returnvalue (AddComponent|AddSceneCaptureComponent2D false))
  (Variables|/Script/Engine.SceneCaptureComponent2D|SetPostProcessSettings _returnvalue (Variables|Default|GetCurrentPostProcess))
  (Variables|/Script/Engine.SceneCaptureComponent2D|SetFOVAngle _returnvalue (Variables|Default|GetCurrentFOV))
  (bind _returnvalue_2 (Rendering|CreateRenderTarget2D _x _y "RTF_RGBA8_SRGB" "(R=0.000000,G=0.000000,B=0.000000,A=1.000000)" true))
  (bind _output_get (Variables|/Script/Engine.SceneCaptureComponent2D|SetTextureTarget _returnvalue _returnvalue_2))
  (Variables|Default|SetRenderTargetTexture _output_get)
  ;[1 1 1] Time to generate the render texture.
  (Utilities|FlowControl|Delay (* 0.1 (Variables|Default|GetCurrentTimeDilation)))
  (Default|UpdateLogoColor (Variables|Default|GetPhotoModeWidgetRef) false)
  ;[1 1 1] Zero-delay. Just to correct the logo colors.
  (Utilities|FlowControl|Delay (Math|Float|MakeLiteralFloat 0.0))
  (Rendering|ExportRenderTarget (Variables|Default|GetRenderTargetTexture) Path Filename)
  (Default|UpdateLogoColor (Variables|Default|GetPhotoModeWidgetRef) true)
  (Utilities|FlowControl|FlipFlop
    (:A
      (Default|MakeThumbnail _photomodewidgetref))
    (:B
      (Default|MakeRegister _photomodewidgetref)
      (Actor|DestroyActor))))

(event EventTick
  (params (DeltaSeconds :type Float%20%28single-precision%29))
  ;[1 1 1] Important for UE4.27+ (to update when paused) even if not used.
)

(fn ConstructionScript
  (Class|Actor|SetTickablewhenPaused true))