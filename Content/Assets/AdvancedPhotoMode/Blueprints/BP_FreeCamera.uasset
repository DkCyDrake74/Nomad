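; Free-flying photo mode camera that moves and rotates from keyboard and gamepad input, interpolated for smoothing.
; Tick applies rotation and swept movement and signals moving or stopped so menu input can be blocked.
; With a maximum distance enabled, it pulls back toward the photo mode component's owner once out of range.
; Construction makes it tick while paused, compensates for global time dilation and applies starting FOV and roll.
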(event EventBeginPlay
  (bind _playercontrollerref (Variables|/Game/Assets/AdvancedPhotoMode/Blueprints/BPC_PhotoMode.BPC_PhotoMode_C|GetPlayerControllerRef (Variables|Default|GetPhotoModeComponentReference))
    (:then
      ;[1 1 1] Enable input for this actor.
      (Input|EnableInput _playercontrollerref))
    (:else)))

(event EventTick
  (params (DeltaSeconds :type Float%20%28single-precision%29))
  (bind (_inputdirection _location _distance) (|CameraMovement DeltaSeconds))
  (Variables|/Game/Assets/AdvancedPhotoMode/Blueprints/BPC_PhotoMode.BPC_PhotoMode_C|GetPlayerControllerRef (Variables|Default|GetPhotoModeComponentReference)
    (:then
      (Transformation|SetActorRotation (|CameraRotation DeltaSeconds))
      (Utilities|FlowControl|Sequence
        (:then_0
          ;[1 1 1] Blocks the menu input while moving.
          (if (> (Math|Float|Absolute(Float) (Math|Vector|VectorLength _inputdirection)) 0.05)
            (Default|CallIsMovingCamera)
            (goto _label Reset)
            (else
              (Utilities|FlowControl|DoOnce false :!label _label
                (:Completed
                  (Default|CallIsNotMovingCamera))))))
        (:then_1
          (if (Variables|Default|GetbUseMaximumDistance)
            (if (< _distance (Variables|Default|GetMaximumDistance))
              (Transformation|SetActorLocation _location true false :!label _label_2)
              (else
                (Transformation|SetActorLocation (Math|Interpolation|VInterpTo (Transformation|GetActorLocation) (+ (* (Math|Rotator|GetRotationXVector (Math|Rotator|FindLookatRotation (Transformation|GetActorLocation) (Transformation|GetActorLocation (Components|GetOwner (Variables|Default|GetPhotoModeComponentReference))))) (Variables|Default|GetMovementSensitivity)) (Transformation|GetActorLocation)) (* DeltaSeconds (Variables|Default|GetCustomTimeDilation)) (Variables|Default|GetMovementInterpolationSpeed)) false false)))
            (else
              (goto _label_2))))))
    (:else)))

(fn ConstructionScript
  (Class|Actor|SetTickablewhenPaused true)
  (Variables|Default|SetCustomTimeDilation (Math|Float|SafeDivide 1.0 (Class|GameplayStatics|GetGlobalTimeDilation)))
  (Camera|SetFieldOfView (Variables|Default|GetCamera) (Variables|Default|GetStartingFOV))
  (Transformation|SetRelativeRotation (Variables|Default|GetCamera) (Math|Rotator|MakeRotator (Variables|Default|GetStartingRoll) 0.0 0.0) false false))