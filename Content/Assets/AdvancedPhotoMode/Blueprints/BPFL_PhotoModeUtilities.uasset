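; Function library for Advanced Photo Mode, with helpers for capture, photo storage and mode state.
; Screenshots and thumbnails use timestamped or derived names, via console commands or a ScreenshotManager render-target export.
; Photo records persist in the PhotosData save slot; other helpers import images and check photo-mode or gallery state.
; Post-process lookup priority-sorts volumes, briefly zeroing each rotation to build oriented boxes for blend-radius camera tests.
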(fn Screenshot(withUI)
  (params (World%20Context%20Object%20%28Self%29 :type Object%20Object%20Reference) (Player%20Controller :type Player%20Controller%20Object%20Reference) (Screenshot%20Folder%20Path :type String))
  (bind _returnvalue (Math|DateTime|Now))
  ;[0.162 0.162 0.162] Take picture of the screen, with UI included (like borders, logo, so remember to hide the PhotoMode Menu!). The resolution corresponds to the size of the window at the time of capture. Returns the path of the created file, useful for use with the "GetScreenshotFile (WithUI)" function.
  (LocalVariables|SetPlayerController Player%20Controller)
  (bind _output_get (LocalVariables|SetFolderPath (Class|BlueprintPathsLibrary|NormalizeDirectoryName Screenshot%20Folder%20Path)))
  (if (Utilities|String|EndsWith _output_get "/")
    _
    (else
      (LocalVariables|SetFolderPath (Utilities|String|Append _output_get "/"))))
  (LocalVariables|SetWorldContextObject World%20Context%20Object%20%28Self%29)
  (bind _output_get_2 (LocalVariables|SetFullFilePath (Utilities|String|Append (LocalVariables|GetFolderPath) (Utilities|String|Append (Utilities|String|ToString(Integer) (.year _returnvalue)) "-" (Utilities|String|ToString(Integer) (.month _returnvalue)) "-" (Utilities|String|ToString(Integer) (.day _returnvalue)) " " (Utilities|String|ToString(Integer) (.hour _returnvalue)) "h" (Utilities|String|ToString(Integer) (.minute _returnvalue)) "min" (Utilities|String|ToString(Integer) (.second _returnvalue)) "s") ".png")))
  (Development|ExecuteConsoleCommand (LocalVariables|GetWorldContextObject) (Utilities|String|Append "Bugscreenshot " _output_get_2) (LocalVariables|GetPlayerController))
  (return (LocalVariables|GetFullFilePath) (Class|BlueprintPathsLibrary|GetBaseFilename _output_get_2 true)))

(fn HighResScreenshot(withoutUI)
  (params (World%20Context%20Object%20%28Self%29 :type Object%20Object%20Reference) (Player%20Controller :type Player%20Controller%20Object%20Reference) (Screenshot%20Folder%20Path :type String) (Resolution%20%28X%20and%20Y%29 :type Int%20Point%20Structure) (ScreenshotMethod :type E_ScreenshotMethod%20Enum :default "NewEnumerator0") (ScreenshotManager :type BP%20Screenshot%20Manager%20Object%20Reference))
  (bind (_x _y) (Utilities|Struct|BreakIntPoint Resolution%20%28X%20and%20Y%29))
  (bind _returnvalue (Math|DateTime|Now))
  (bind _returnvalue_2 (Utilities|String|ToString(Integer) _x))
  (bind _returnvalue_3 (Utilities|String|ToString(Integer) (.day _returnvalue)))
  (bind _returnvalue_4 (Utilities|String|ToString(Integer) _y))
  (bind _returnvalue_5 (Utilities|String|ToString(Integer) (.hour _returnvalue)))
  (bind _returnvalue_6 (Utilities|String|ToString(Integer) (.minute _returnvalue)))
  (bind _returnvalue_7 (Utilities|String|ToString(Integer) (.second _returnvalue)))
  (bind _returnvalue_8 (Utilities|String|ToString(Integer) (.year _returnvalue)))
  (bind _returnvalue_9 (Utilities|String|ToString(Integer) (.month _returnvalue)))
  (bind _returnvalue_10 (Utilities|String|Append _returnvalue_2 "x" _returnvalue_4))
  (bind _returnvalue_11 (Utilities|String|Append _returnvalue_8 "-" _returnvalue_9 "-" _returnvalue_3 " " _returnvalue_5 "h" _returnvalue_6 "min" _returnvalue_7 "s" "_" _returnvalue_10))
  (bind _returnvalue_12 (Utilities|String|Append _returnvalue_11 ".png"))
  ;[0.162 0.162 0.162] Take picture of the screen, but without UI included (but it can capture borders and logos of Advanced Photo Mode). You can decide the resolution. Returns the path of the created file, useful for use with the "GetHighResScreenshotFile (without UI)" function.
  (LocalVariables|SetPlayerController Player%20Controller)
  (LocalVariables|SetResolution _returnvalue_10)
  (bind _output_get (LocalVariables|SetFolderPath (Class|BlueprintPathsLibrary|NormalizeDirectoryName Screenshot%20Folder%20Path)))
  (if (Utilities|String|EndsWith _output_get "/")
    _
    (else
      (LocalVariables|SetFolderPath (Utilities|String|Append _output_get "/"))))
  (LocalVariables|SetWorldContextObject World%20Context%20Object%20%28Self%29)
  (bind _output_get_2 (LocalVariables|SetFullFilePath (Utilities|String|Append (LocalVariables|GetFolderPath) _returnvalue_12)))
  (switch Utilities|FlowControl|Switch|SwitchonE_ScreenshotMethod ScreenshotMethod
    (:NewEnumerator0
      (Development|ExecuteConsoleCommand (LocalVariables|GetWorldContextObject) (Utilities|String|Append "HighResShot " (LocalVariables|GetResolution) " filename=\"" _output_get_2 "\"") (LocalVariables|GetPlayerController)))
    (:NewEnumerator1
      (bind _screenshotmanager (LocalVariables|GetScreenshotManager)
        (:then
          (Default|TakeScreenshot _screenshotmanager Resolution%20%28X%20and%20Y%29 (LocalVariables|GetFolderPath) _returnvalue_12))
        (:else))))
  (return (LocalVariables|GetFullFilePath) (Class|BlueprintPathsLibrary|GetBaseFilename _output_get_2 true)))

(fn GetDefaultScreenResolution
  (bind _returnvalue (Viewport|GetViewportSize))
  ;[0.162 0.162 0.162] Returns the user's screen resolution, or a multiple standard resolution (1920x1080).
  (return (Class|KismetMathLibrary|ToIntPoint(Vector2D) (select (Math|Vector|Equal(Vector) :A _returnvalue) "(X=1920.000000,Y=1080.000000)" _returnvalue))))

(fn DirectoryPathCorrection
  (params (Use%20Custom%20Path? :type Boolean) (Custom%20Path :type String))
  ;[0.162 0.162 0.162] Corrects the directory path, that is, if the directory does not exist, makes the path the default.
  (return (Utilities|String|SelectString Custom%20Path (Class|BlueprintPathsLibrary|RemoveDuplicateSlashes (Class|BlueprintPathsLibrary|NormalizeDirectoryName (Utilities|String|Append (Class|BlueprintPathsLibrary|ProjectDir) "/Screenshots/"))) (and Use%20Custom%20Path? (not (Utilities|Text|TextIsEmpty (Utilities|Text|ToText(String) Custom%20Path)))))))

(fn GetScreenshotFile
  (params (WorldContextObject :type Object%20Object%20Reference) (FullFilePath :type String))
  ;[0.162 0.162 0.162] Capture the photo from the provided folder. Returns whether the image is valid, the image, its name and its path.
  (if (Class|BlueprintPathsLibrary|FileExists FullFilePath)
    (bind _returnvalue (Class|KismetRenderingLibrary|ImportFileasTexture2D WorldContextObject FullFilePath))
    (return (Utilities|IsValid _returnvalue) _returnvalue (Class|BlueprintPathsLibrary|GetBaseFilename FullFilePath true) FullFilePath)
    (else
      (return false 0 "" ""))))

(fn NormalizeScreenshotPath
  (params (Folder%20Path :type String))
  ;[0.162 0.162 0.162] Normalizes the directory name based on the Unreal Engine.
  (bind _output_get (LocalVariables|SetFolderPath (Class|BlueprintPathsLibrary|NormalizeDirectoryName Folder%20Path)))
  (if (Utilities|String|EndsWith _output_get "/")
    _
    (else
      (LocalVariables|SetFolderPath (Utilities|String|Append _output_get "/"))))
  (return (LocalVariables|GetFolderPath)))

(fn SavePhoto
  (params (SaveNewPhoto :type S%20Photos%20Data%20Structure) (Sort :type E_SaveSort%20Enum :default "NewEnumerator0"))
  (bind _returnvalue (SaveGame|LoadGamefromSlot "PhotosData"))
  (bind _assg_photos_data_save_game (Utilities|Casting|CastToSG_PhotosDataSaveGame _returnvalue)
    (:then
      ;[1 1 1] If save game already exists, we use it.
      (LocalVariables|SetSaveGameReference _assg_photos_data_save_game))
    (:CastFailed
      ;[1 1 1] If save game doesn't exists, we create one.
      (bind _returnvalue_2 (SaveGame|CreateSaveGameObject "/Game/Assets/AdvancedPhotoMode/SaveGame/SG_PhotosDataSaveGame.SG_PhotosDataSaveGame_C"))
      (LocalVariables|SetSaveGameReference _returnvalue_2)))
  (switch Utilities|FlowControl|Switch|SwitchonE_SaveSort Sort
    (:NewEnumerator0
      (Utilities|Array|Insert (Variables|/Game/Assets/AdvancedPhotoMode/SaveGame/SG_PhotosDataSaveGame.SG_PhotosDataSaveGame_C|GetPhotosData (LocalVariables|GetSaveGameReference)) SaveNewPhoto))
    (:NewEnumerator1
      (Utilities|Array|AddUnique (Variables|/Game/Assets/AdvancedPhotoMode/SaveGame/SG_PhotosDataSaveGame.SG_PhotosDataSaveGame_C|GetPhotosData (LocalVariables|GetSaveGameReference)) SaveNewPhoto)))
  (SaveGame|SaveGametoSlot (LocalVariables|GetSaveGameReference) "PhotosData"))

(fn LoadPhotos
  ;[0.162 0.162 0.162] Load the photos information
  (bind _returnvalue (SaveGame|LoadGamefromSlot "PhotosData"))
  (bind _assg_photos_data_save_game (Utilities|Casting|CastToSG_PhotosDataSaveGame _returnvalue)
    (:then
      (return true (Variables|/Game/Assets/AdvancedPhotoMode/SaveGame/SG_PhotosDataSaveGame.SG_PhotosDataSaveGame_C|GetPhotosData _assg_photos_data_save_game)))
    (:CastFailed
      (return false 0))))

(fn MakeThumbnail
  (params (World%20Context%20Object%20%28Self%29 :type Object%20Object%20Reference) (Player%20Controller :type Player%20Controller%20Object%20Reference) (Screenshot%20Folder%20Path :type String) (Resolution%20%28X%20and%20Y%29 :type Int%20Point%20Structure) (PhotoName :type String) (ScreenshotMethod :type E_ScreenshotMethod%20Enum :default "NewEnumerator0") (ScreenshotManager :type BP%20Screenshot%20Manager%20Object%20Reference))
  (bind (_x _y) (Utilities|Struct|BreakIntPoint Resolution%20%28X%20and%20Y%29))
  (bind _returnvalue (Utilities|String|Append PhotoName "_thumbnail"))
  (bind _returnvalue_2 (Utilities|String|Append _returnvalue ".png"))
  ;[0.162 0.162 0.162] Take picture of the screen, but without UI included (but it can capture borders and logos of Advanced Photo Mode). You can decide the resolution. Returns the path of the created file, useful for use with the "GetHighResScreenshotFile (without UI)" function.
  (LocalVariables|SetPlayerController Player%20Controller)
  (LocalVariables|SetResolution (Utilities|String|Append (Utilities|String|ToString(Integer) _x) "x" (Utilities|String|ToString(Integer) _y)))
  (bind _output_get (LocalVariables|SetFolderPath (Class|BlueprintPathsLibrary|NormalizeDirectoryName Screenshot%20Folder%20Path)))
  (if (Utilities|String|EndsWith _output_get "/")
    _
    (else
      (LocalVariables|SetFolderPath (Utilities|String|Append _output_get "/"))))
  (LocalVariables|SetFolderPath (Utilities|String|Append (LocalVariables|GetFolderPath) "thumbnails/"))
  (LocalVariables|SetWorldContextObject World%20Context%20Object%20%28Self%29)
  (bind _output_get_2 (LocalVariables|SetFullFilePath (Utilities|String|Append (LocalVariables|GetFolderPath) _returnvalue_2)))
  (switch Utilities|FlowControl|Switch|SwitchonE_ScreenshotMethod ScreenshotMethod
    (:NewEnumerator0
      (Development|ExecuteConsoleCommand (LocalVariables|GetWorldContextObject) (Utilities|String|Append "HighResShot " (LocalVariables|GetResolution) " filename=\"" _output_get_2 "\"") (LocalVariables|GetPlayerController)))
    (:NewEnumerator1
      (bind _screenshotmanager (LocalVariables|GetScreenshotManager)
        (:then
          (Default|TakeScreenshot _screenshotmanager Resolution%20%28X%20and%20Y%29 (LocalVariables|GetFolderPath) _returnvalue_2))
        (:else))))
  (return (LocalVariables|GetFullFilePath) (Class|BlueprintPathsLibrary|GetBaseFilename _output_get_2 true)))

(fn SaveAllPhotos
  (params (SaveNewPhoto :type Array%20of%20S%20Photos%20Data%20Structures))
  ;[0.162 0.162 0.162] Save all photos information
  (bind _returnvalue (SaveGame|LoadGamefromSlot "PhotosData"))
  (bind _assg_photos_data_save_game (Utilities|Casting|CastToSG_PhotosDataSaveGame _returnvalue)
    (:then
      ;;[1 1 1] If save game already exists, we use it.
      (LocalVariables|SetSaveGameReference _assg_photos_data_save_game))
    (:CastFailed
      ;;[1 1 1] If save game doesn't exists, we create one.
      (bind _returnvalue_2 (SaveGame|CreateSaveGameObject "/Game/Assets/AdvancedPhotoMode/SaveGame/SG_PhotosDataSaveGame.SG_PhotosDataSaveGame_C"))
      (LocalVariables|SetSaveGameReference _returnvalue_2)))
  (Variables|/Game/Assets/AdvancedPhotoMode/SaveGame/SG_PhotosDataSaveGame.SG_PhotosDataSaveGame_C|SetPhotosData (LocalVariables|GetSaveGameReference) SaveNewPhoto)
  (SaveGame|SaveGametoSlot (LocalVariables|GetSaveGameReference) "PhotosData"))

(fn HideHUDwhenUsingPhotoMode
  (params (If%20Not%20Using%20Photo%20Mode%20Set%20This%20Widget%20As :type ESlateVisibility%20Enum :default "Visible") (PhotoModeComponent :type BPC%20Photo%20Mode%20Object%20Reference))
  (bind _bisusinggallery (Variables|/Game/Assets/AdvancedPhotoMode/Blueprints/BPC_PhotoMode.BPC_PhotoMode_C|GetbIsUsingGallery PhotoModeComponent))
  (bind _bisusingphotomode (Variables|/Game/Assets/AdvancedPhotoMode/Blueprints/BPC_PhotoMode.BPC_PhotoMode_C|GetbIsUsingPhotoMode PhotoModeComponent))
  (bind _returnvalue (or _bisusinggallery _bisusingphotomode))
  ;[0.162 0.162 0.162] You can use this function to hide your HUD elements creating a bind function in the main canvas panel of your widget using this function!
  (Utilities|IsValid PhotoModeComponent
    (:Is%20Valid
      (return (select _returnvalue "Hidden" If%20Not%20Using%20Photo%20Mode%20Set%20This%20Widget%20As) _returnvalue))
    (:Is%20Not%20Valid
      (return If%20Not%20Using%20Photo%20Mode%20Set%20This%20Widget%20As false))))

(fn NearestDistancetoBoxwithTransform
  (params (Point :type Vector) (BoxWorldTransform :type Transform) (BoxExtent :type Vector))
  (bind _returnvalue (Math|Transform|InverseTransformLocation BoxWorldTransform Point))
  (bind (_x _y _z) (Math|Vector|BreakVector _returnvalue))
  ;[1 1 1] Given a point in space and a box volume (its origin and extent), returns the closest distance between the point and the volume surface.
  (LocalVariables|SetBox (Math|Box|MakeBox (* BoxExtent -1) BoxExtent))
  (return (Math|Float|Sqrt (+ (* (Math|Vector|GetMaxElement (Math|Vector|MakeVector (- (.X (Math|Vector|BreakVector (.Min (Utilities|Struct|BreakBox (LocalVariables|GetBox))))) _x) (- _x (.X (Math|Vector|BreakVector (.Max (Utilities|Struct|BreakBox (LocalVariables|GetBox)))))) 0.0)) (Math|Vector|GetMaxElement (Math|Vector|MakeVector (- (.X (Math|Vector|BreakVector (.Min (Utilities|Struct|BreakBox (LocalVariables|GetBox))))) _x) (- _x (.X (Math|Vector|BreakVector (.Max (Utilities|Struct|BreakBox (LocalVariables|GetBox)))))) 0.0))) (* (Math|Vector|GetMaxElement (Math|Vector|MakeVector (- (.Y (Math|Vector|BreakVector (.Min (Utilities|Struct|BreakBox (LocalVariables|GetBox))))) _y) (- _y (.Y (Math|Vector|BreakVector (.Max (Utilities|Struct|BreakBox (LocalVariables|GetBox)))))) 0.0)) (Math|Vector|GetMaxElement (Math|Vector|MakeVector (- (.Y (Math|Vector|BreakVector (.Min (Utilities|Struct|BreakBox (LocalVariables|GetBox))))) _y) (- _y (.Y (Math|Vector|BreakVector (.Max (Utilities|Struct|BreakBox (LocalVariables|GetBox)))))) 0.0))) (* (Math|Vector|GetMaxElement (Math|Vector|MakeVector (- (.Z (Math|Vector|BreakVector (.Min (Utilities|Struct|BreakBox (LocalVariables|GetBox))))) _z) (- _z (.Z (Math|Vector|BreakVector (.Max (Utilities|Struct|BreakBox (LocalVariables|GetBox)))))) 0.0)) (Math|Vector|GetMaxElement (Math|Vector|MakeVector (- (.Z (Math|Vector|BreakVector (.Min (Utilities|Struct|BreakBox (LocalVariables|GetBox))))) _z) (- _z (.Z (Math|Vector|BreakVector (.Max (Utilities|Struct|BreakBox (LocalVariables|GetBox)))))) 0.0)))))))

(fn GetAllImersedPostProcess
  (params (PlayerController :type Player%20Controller%20Object%20Reference))
  ;[1 1 1] Finds and returns all post process volumes that the player is immersed in.
  (LocalVariables|SetCameraLoc (Transformation|GetActorLocation (Variables|/Script/Engine.PlayerController|GetPlayerCameraManager PlayerController)))
  (bind _outactors (Actor|GetAllActorsOfClass 0 "/Script/Engine.PostProcessVolume"))
  (bind _output_get (LocalVariables|SetPostProcessVolumes _outactors))
  (for _array_element _output_get
    (Utilities|Array|Add (LocalVariables|GetPriorityArray) (Variables|/Script/Engine.PostProcessVolume|GetPriority _array_element)))
  (bind _output_get_2 (LocalVariables|SetLastIndex (Utilities|Array|LastIndex _output_get)))
  (for _index (range 1 _output_get_2)
    (for _index_2 (range 0 (- (LocalVariables|GetLastIndex) _index))
      (if (> (Utilities|Array|Get(acopy) (LocalVariables|GetPriorityArray) _index_2) (Utilities|Array|Get(acopy) (LocalVariables|GetPriorityArray) (+ _index_2 1)))
        (Utilities|Array|Swap (LocalVariables|GetPriorityArray) _index_2 (+ _index_2 1))
        (Utilities|Array|Swap (LocalVariables|GetPostProcessVolumes) _index_2 (+ _index_2 1)))))
  (for _array_element_2 (LocalVariables|GetPostProcessVolumes)
    (LocalVariables|SetCurrentPostProcessRotation (Transformation|GetActorRotation _array_element_2))
    (Utilities|FlowControl|Sequence
      (:then_0
        (Transformation|SetActorRotation _array_element_2)
        (LocalVariables|SetBoxTransform (Math|Transform|MakeTransform (.Origin (Collision|GetActorBounds _array_element_2 false false)) (LocalVariables|GetCurrentPostProcessRotation)))
        ;;[1 1 1] Check if the camera is within the PP volume, counting the blend radius.
        (LocalVariables|SetBoxExtent (.BoxExtent (Collision|GetActorBounds _array_element_2 false false)))
        (if (and (Variables|/Script/Engine.PostProcessVolume|GetbEnabled _array_element_2) (or (Variables|/Script/Engine.PostProcessVolume|GetbUnbound _array_element_2) (Class|KismetMathLibrary|IsPointinBoxwithTransform (LocalVariables|GetCameraLoc) (LocalVariables|GetBoxTransform) (+ (.BoxExtent (Collision|GetActorBounds _array_element_2 false false)) (Variables|/Script/Engine.PostProcessVolume|GetBlendRadius _array_element_2)))))
          (Utilities|Map|Add (LocalVariables|GetBlendedPostProcessVolumes) _array_element_2 (LocalVariables|GetBoxTransform))
          (Utilities|Map|Add (LocalVariables|GetBlendedVolumesExtent) _array_element_2 (LocalVariables|GetBoxExtent))))
      (:then_1
        (Transformation|SetActorRotation _array_element_2 (LocalVariables|GetCurrentPostProcessRotation)))))
  (return (LocalVariables|GetCameraLoc) (LocalVariables|GetBlendedPostProcessVolumes) (LocalVariables|GetBlendedVolumesExtent)))

(fn IsPhotoModeOpened
  (bind _foundwidgets (Widget|GetAllWidgetsOfClass 0 "/Game/Assets/AdvancedPhotoMode/Blueprints/UI_PhotoMode.UI_PhotoMode_C" false))
  (if (Utilities|Array|IsValidIndex _foundwidgets)
    (return true (Utilities|Array|Get(acopy) _foundwidgets))
    (else
      (return false 0))))

(fn IsGalleryOpened
  (bind _foundwidgets (Widget|GetAllWidgetsOfClass 0 "/Game/Assets/AdvancedPhotoMode/Blueprints/UI_Gallery.UI_Gallery_C" false))
  (if (Utilities|Array|IsValidIndex _foundwidgets)
    (return true (Utilities|Array|Get(acopy) _foundwidgets))
    (else
      (return false 0))))

(fn IsPhotoModeorGalleryOpened
  (return (or (.bIsOpened (AdvancedPhotoMode|IsPhotoModeOpened)) (.bIsOpened (AdvancedPhotoMode|IsGalleryOpened)))))