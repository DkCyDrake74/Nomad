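; Loot box Blueprint that rolls a random item from a loot data table when play begins.
; GenerateLoot reads the table's row names, accumulates DropChance into a total and draws a random integer up to that total.
; That integer directly indexes the row names, without a cumulative weight lookup, and the selected row's Item class name is printed.
; Tick prints the rolled value on screen as debug output.
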(event EventBeginPlay
  (CallFunction|GenerateLoot))

(event Collision|EventActorBeginOverlap
  (params (OtherActor :type Actor%20Object%20Reference)))

(event EventTick
  (params (DeltaSeconds :type Float%20%28single-precision%29))
  (Development|PrintString (Utilities|String|ToString(Integer) (Variables|Default|GetRandomValue)) true true "(R=0.000000,G=1.000000,B=0.000000,A=1.000000)" 0.001))

(fn ConstructionScript)

(fn GenerateLoot
  (bind _outrownames (DataTable|GetDataTableRowNames (Variables|Default|GetDT_LootTable)))
  (bind _output_get (LocalVariables|SetNames _outrownames))
  (for _array_element _output_get
    _)
  (bind _returnvalue (Utilities|GetDataTableRow "/Game/Inventory/Loot/DT_LootTable.DT_LootTable" _array_element)
    (:then
      (bind _output_get_2 (Variables|Default|SetTotalDropChance (+ (.dropchance _returnvalue) (Variables|Default|GetTotalDropChance))))
      (bind _output_get_3 (Variables|Default|SetRandomValue (Math|Random|RandomIntegerinRange 0 _output_get_2)))
      (bind _returnvalue_2 (Utilities|GetDataTableRow "/Game/Inventory/Loot/DT_LootTable.DT_LootTable" (Utilities|Array|Get(acopy) (LocalVariables|GetNames) _output_get_3))
        (:then
          (Development|PrintString (Utilities|GetClassDisplayName (.item _returnvalue_2))))))))