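; BP_M4A1 is an M4A1 weapon pickup that equips itself when the third-person character overlaps its box.
; The overlap flags the weapon as equipped on both the character and its AB_Player anim instance, then snaps the weapon to the mesh's WeaponPosition socket.
; A separate AmmoSpawn function spawns a BP_Ammo actor at the Sphere component's world transform.
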(event OnComponentBeginOverlap(Box)
  (params (OverlappedComponent :type Primitive%20Component%20Object%20Reference) (OtherActor :type Actor%20Object%20Reference) (OtherComp :type Primitive%20Component%20Object%20Reference) (OtherBodyIndex :type Integer) (bFromSweep :type Boolean) (SweepResult :type Hit%20Result%20Structure%20%28by%20ref%29))
  (bind _asbp_third_person_character (Utilities|Casting|CastToBP_ThirdPersonCharacter OtherActor))
  (Variables|/Game/ThirdPerson/Blueprints/BP_ThirdPersonCharacter.BP_ThirdPersonCharacter_C|SetWeaponIsEquip _asbp_third_person_character true)
  (bind _asab_player (Utilities|Casting|CastToAB_Player (Components|SkeletalMesh|GetAnimInstance (Variables|/Script/Engine.Character|GetMesh _asbp_third_person_character))))
  (Variables|/Game/Player/AB_Player.AB_Player_C|SetWeaponEquip _asab_player true)
  (Transformation|AttachComponentToComponent (Variables|/Script/Engine.Character|GetMesh _asbp_third_person_character) "WeaponPosition" "SnapToTarget" "SnapToTarget" "SnapToTarget" true))

(event EventBeginPlay)

(event Collision|EventActorBeginOverlap
  (params (OtherActor :type Actor%20Object%20Reference)))

(event EventTick
  (params (DeltaSeconds :type Float%20%28single-precision%29)))

(fn ConstructionScript)

(fn AmmoSpawn
  (Game|SpawnActorfromClass "/Game/Weapon/M4A1/BP_Ammo.BP_Ammo_C" (Transformation|GetWorldTransform (Variables|Default|GetSphere)) "Undefined" "MultiplyWithRoot" 0 0))